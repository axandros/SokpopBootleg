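; Villager unit Blueprint that extends a parent unit class with a timed revival after death.
; The construction script sets a fixed attack range, and the OnDeath override runs the parent logic, then starts a one-shot timer lasting DeathTime.
; OnDeathTimerOver, apparently that timer's callback, restores minimal health and switches movement back to NavWalking.
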(event Custom|OnDeathTimerOver
  (Variables|Default|SetHealth 1)
  (Pawn|Components|CharacterMovement|SetMovementMode (Variables|Character|GetCharacterMovement) "MOVE_NavWalking" 0))

(event EventBeginPlay
  (|CallParentFunction) ; This node is disabled and will not be called.\nDrag off pins to build functionality.
)

(event Collision|EventActorBeginOverlap
  (params (OtherActor :type Actor%20Object%20Reference))
  (|CallParentFunction OtherActor) ; This node is disabled and will not be called.\nDrag off pins to build functionality.
)

(event EventTick
  (params (DeltaSeconds :type Float%20%28single-precision%29))
  (|CallParentFunction DeltaSeconds) ; This node is disabled and will not be called.\nDrag off pins to build functionality.
)

(fn ConstructionScript
  (|CallParentFunction)
  (Variables|Default|SetAttackRange 1.5e+03))

(fn OnDeath
  (|CallParentFunction)
  (Utilities|Time|SetTimerbyEvent (EventDispatchers|CreateEvent :!event Custom|OnDeathTimerOver) (Variables|Default|GetDeathTime)))